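; Abstract event trigger actor that activates, deactivates or switches a target Object when certain actors enter its box collider.
; Overlaps count only when the other actor's class exactly matches an entry in TriggerActors.
; A DoOnce gate, reset after ReloadTime, prevents repeated interactions.
; Interact plays a 2D sound and runs the action selected by Type, or prints an error if Object is invalid.
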(event OnComponentBeginOverlap(BoxCollider)
  (params (OverlappedComponent :type Primitive%20Component%20Object%20Reference) (OtherActor :type Actor%20Object%20Reference) (OtherComp :type Primitive%20Component%20Object%20Reference) (OtherBodyIndex :type Integer) (bFromSweep :type Boolean) (SweepResult :type Hit%20Result%20Structure%20%28by%20ref%29))
  ;[0 0 0] Interact only with Actors from the list
  (for _array_element (Variables|Params|GetTriggerActors)
    (if (== _array_element (Utilities|GetClass OtherActor))
      ;[0 0 0] Interact with delay for preventing multiple Interactions
      (Utilities|FlowControl|DoOnce false :!label _label
        (:Completed
          (CallFunction|Interact)
          (Utilities|FlowControl|Delay (Variables|Params|GetReloadTime))
          (goto _label Reset))))))

(fn ConstructionScript)

(fn Interact
  (bind _object (Variables|Params|GetObject))
  ;[0 0 0] Make action depending on Type
  (Utilities|IsValid (Variables|Params|GetObject)
    (:Is%20Valid
      (Audio|PlaySound2D (Variables|Params|GetSound) 1.0 1.0 0.0 0 0)
      (switch Utilities|FlowControl|Switch|SwitchonEventTriggerTypes_Enum (Variables|Params|GetType)
        (:NewEnumerator0
          (Default|Activate _object))
        (:NewEnumerator1
          (Default|Deactivate _object))
        (:NewEnumerator2
          (Default|Switch _object))))
    (:Is%20Not%20Valid
      (Development|PrintString "Object Is not set In Event Trigger!" true true "(R=1.000000,G=0.029525,B=0.000000,A=1.000000)"))))