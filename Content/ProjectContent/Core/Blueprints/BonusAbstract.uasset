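; BonusAbstract is a base actor for bonus pickups that the player collects by touching them.
; Tick spins the static mesh around its yaw axis at RotationSpeed, scaled by delta time.
; The box overlap passes only Player actors to Pickup, which plays a 2D sound and destroys the bonus.
; Pickup receives the player reference but applies no effect to it here.
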(event OnComponentBeginOverlap(Box)
  (params (OverlappedComponent :type Primitive%20Component%20Object%20Reference) (OtherActor :type Actor%20Object%20Reference) (OtherComp :type Primitive%20Component%20Object%20Reference) (OtherBodyIndex :type Integer) (bFromSweep :type Boolean) (SweepResult :type Hit%20Result%20Structure%20%28by%20ref%29))
  ;[0 0 0] Pickup the Bonus By Player
  (bind _asplayer (Utilities|Casting|CastToPlayer OtherActor))
  (CallFunction|Pickup _asplayer))

(event EventTick
  (params (DeltaSeconds :type Float%20%28single-precision%29))
  (bind _staticmesh (Variables|Default|GetStaticMesh))
  (bind _returnvalue (Transformation|GetWorldRotation _staticmesh))
  ;[0 0 0] Static Mesh Rotation
  (Transformation|SetWorldRotation (Variables|Default|GetStaticMesh) (Math|Rotator|MakeRotator (.roll _returnvalue) (.pitch _returnvalue) (+ (.yaw _returnvalue) (* DeltaSeconds (Variables|Default|GetRotationSpeed)))) false false))

(fn ConstructionScript)

(fn Pickup
  (params (PlayerRef :type Player%20Object%20Reference))
  (Audio|PlaySound2D (Variables|Default|GetPickupSound) 0.8 1.0 0.0 0 0)
  (Actor|DestroyActor))