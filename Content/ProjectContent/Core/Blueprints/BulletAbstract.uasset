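; BulletAbstract is a bullet Blueprint, named as an abstract base, that provides lifetime, scale and trace behavior.
; The construction script applies a uniform Scale to the Scene component, and BeginPlay sets a lifespan so bullets that miss are removed.
; ForwardLineTrace returns a Visibility-channel hit from the actor's location over a given distance, along world forward (zero rotation) rather than the actor's facing.
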(event EventBeginPlay
  ;[1 1 1 1 20] Remove bullet if not hit
  (if (Utilities|IsValid self)
    (Actor|SetLifeSpan (Variables|Default|GetBulletLifeSpan))))

(fn ConstructionScript
  (bind _scale (Variables|Default|GetScale))
  (Transformation|SetWorldScale3D (Variables|Default|GetScene) (Math|Vector|MakeVector _scale _scale _scale)))

(fn ForwardLineTrace
  (params (Distance :type Float%20%28single-precision%29))
  (bind _returnvalue (Transformation|GetActorLocation))
  (bind _outhit (Collision|LineTraceByChannel _returnvalue (+ _returnvalue (* (Math|Vector|GetForwardVector "0, 0, 0") Distance)) "TraceTypeQuery1" false 0 "None"))
  (return _outhit))