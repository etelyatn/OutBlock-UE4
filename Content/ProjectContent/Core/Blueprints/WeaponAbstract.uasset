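; Base weapon Blueprint for the player that handles firing, ammo, magazines and reloading.
; Shooting plays a montage and fires either one shot or repeatedly on a looping timer when auto-fire is set.
; Each shot traces from the follow camera with random spread, then spawns a bullet at the muzzle socket aimed at the impact point or trace end.
; An empty magazine triggers a timed reload, or notifies the player when none remain.
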(event Custom|OnMagOutOfAmo
  ;[0 0 0] Mag Out Of Amo
  (CallFunction|OnStopShooting)
  ;;[0 0 0] If have mags - reloading
  (if (> (Variables|Default|GetCurrentMags) 0)
    (CallFunction|OnReloading)
    (else
      ;;[0 0 0] Inform Player Out of Ammo
      (Default|OnOutOfAmmo (Variables|Default|GetPlayerRef))
      (Development|PrintString "OutOfAmmo"))))

(event Custom|OnReloading
  (Math|Integer|DecrementInt (Variables|Default|GetCurrentMags)
    (:%20%20
      (Variables|Default|SetIsReloading true)
      (Development|PrintString "Reloading")
      (Animation|Montage|MontagePlay (Default|GetPlayerAnimInstance (Variables|Default|GetPlayerRef)) (Variables|Animations|GetReloadAnim) 1.0 "MontageLength" 0.0 true)
      (Audio|PlaySound2D (Variables|Stats|GetReloadSound) 1.0 1.0 0.0 0 0)
      (Utilities|FlowControl|Delay (Variables|Stats|GetReloadTime))
      (Variables|Default|SetCurrentAmmo (Variables|Stats|GetMaxAmmo))
      (Variables|Default|SetIsReloading false)
      (Development|PrintString "Reloading Finished"))))

(event EventBeginPlay
  ;[0 0 0] Save Player Reference
  (bind _asplayer (Utilities|Casting|CastToPlayer (Game|GetPlayerCharacter 0)))
  (Variables|Default|SetPlayerRef _asplayer))

(event EventShootingBegin
  ;[0 0 0] Shooting Events
  (|ShootingGraph))

(event EventShootingEnd
  ;[0 0 0] Shooting Events
  (CallFunction|OnStopShooting))

(fn GetShootingTrace
  (params (Distance :type Float%20%28single-precision%29) (SpreadDistance :type Float%20%28single-precision%29) (DrawDebug :type EDrawDebugTrace%20Enum :default "None"))
  (bind _self self)
  (bind _returnvalue (Transformation|GetSocketTransform _self "MuzzleSocket" "RTS_World"))
  ;[0 0 0] Line trace for shooting
  (bind _outhit (Collision|LineTraceByChannel (Transformation|GetWorldLocation (Variables|/Game/ProjectContent/Blueprints/Player.Player_C|GetFollowCamera (Variables|Default|GetPlayerRef))) (+ (CallFunction|GetTraceDistance Distance) (CallFunction|GetBulletSpreadAmount SpreadDistance)) "TraceTypeQuery1" false 0 DrawDebug true "(R=1.000000,G=0.000000,B=0.000000,A=1.000000)" "(R=0.000000,G=1.000000,B=0.000000,A=1.000000)" 1.0))
  ;[0 0 0] Outputs added from the line trace so that they can be used to calculate projectile details
  (return (.bBlockingHit (Collision|BreakHitResult _outhit)) (.HitActor (Collision|BreakHitResult _outhit)) (.HitComponent (Collision|BreakHitResult _outhit)) (.Normal (Collision|BreakHitResult _outhit)) (Collision|GetSurfaceType _outhit) (.TraceStart (Collision|BreakHitResult _outhit)) (.TraceEnd (Collision|BreakHitResult _outhit)) (Math|Transform|MakeTransform (.location _returnvalue) (Math|Rotator|FindLookatRotation (.location _returnvalue) (Math|Vector|SelectVector (.ImpactPoint (Collision|BreakHitResult _outhit)) (.TraceEnd (Collision|BreakHitResult _outhit)) (.bBlockingHit (Collision|BreakHitResult _outhit)))))))

(fn GetTraceDistance
  (params (Distance :type Float%20%28single-precision%29))
  (bind _playerref (Variables|Default|GetPlayerRef))
  (bind _followcamera (Variables|/Game/ProjectContent/Blueprints/Player.Player_C|GetFollowCamera _playerref))
  (return (+ (Transformation|GetWorldLocation _followcamera) (* (Math|Vector|GetForwardVector _followcamera) Distance))))

(fn GetBulletSpreadAmount
  (params (SpreadDistance :type Float%20%28single-precision%29))
  (bind (_negative _positive) (CallFunction|GetNegativeandPositive SpreadDistance))
  (return (Math|Vector|MakeVector (Math|Random|RandomFloatinRange _negative _positive) (Math|Random|RandomFloatinRange _negative _positive) (Math|Random|RandomFloatinRange _negative _positive))))

(fn SpawnBullet
  (params (SpawnTransform :type Transform) (HitNormal :type Vector))
  (bind _returnvalue (Game|SpawnActorfromClass (Variables|Default|GetBulletClass) SpawnTransform "Undefined" 0 1.0 HitNormal 0))
  (Audio|PlaySound2D (Variables|/Game/ProjectContent/Core/Blueprints/BulletAbstract.BulletAbstract_C|GetSound _returnvalue) 1.0 1.0 0.0 0 0)
  (Effects|SpawnEmitterAttached (Variables|/Game/ProjectContent/Core/Blueprints/BulletAbstract.BulletAbstract_C|GetStartVFX _returnvalue) self "MuzzleSocket" "0, 0, 0" "0.000000,90.000000,0.000000" "0.500000,0.500000,0.500000"))

(fn GetCurrentAmmo
  (return (Variables|Default|GetCurrentAmmo)))

(fn HasAmmo
  (return (or (> (Variables|Default|GetCurrentAmmo) 0) (> (Variables|Default|GetCurrentMags) 0))))

(fn IsShootingValid
  (return (Math|Boolean|ANDBoolean (not (Variables|Default|GetIsShooting)) (not (Variables|Default|GetIsReloading)) (> (Variables|Default|GetCurrentAmmo) 0))))

(fn GetMagsAmmo
  (return (* (Variables|Default|GetCurrentMags) (Variables|Stats|GetMaxAmmo))))

(event Custom|OnShootBullet
  ;[0 0 0] One Shoot Event
  ;;[0 0 0] Check If have Ammo and decrement it
  (if (> (Variables|Default|GetCurrentAmmo) 0)
    (Math|Integer|DecrementInt (Variables|Default|GetCurrentAmmo)
      (:%20%20
        ;;[0 0 0] Shoot Bullet Event. Spawn a bullet by Trace
        (bind (_bblockinghit _hitactor _hitcomponent _normal _hitsurface _tracestart _traceend _spawntransform) (CallFunction|GetShootingTrace 3.5e+03 4e+01 "None"))
        (CallFunction|SpawnBullet _spawntransform _normal)
        ;;[0 0 0] Call when out of Ammo
        (if (<= (Variables|Default|GetCurrentAmmo) 0)
          (CallFunction|OnMagOutOfAmo))))))

(event Custom|OnStopShooting
  (bind _autofirehandle (Variables|Default|GetAutoFireHandle))
  ;[0 0 0] Stop Shooting
  ;;[0 0 0] Stop Shooting animation
  (Animation|Montage|MontageStop (Default|GetPlayerAnimInstance (Variables|Default|GetPlayerRef)) 0.2 (Variables|Animations|GetShootAnim))
  ;;[0 0 0] Disable Shooting process
  (if (Variables|Default|GetIsShooting)
    (Variables|Default|SetIsShooting false)
    ;;[0 0 0] Clear Autoshooting timer
    (if (Utilities|Time|IsValidTimerHandle _autofirehandle)
      (Utilities|Time|ClearandInvalidateTimerbyHandle _autofirehandle))))

(event Custom|AutoFiringEvent
  ;[0 0 0] Start Shooting
  ;;[0 0 0] Enable Autofire (Few shoots when the fire button on hold)
  (CallFunction|OnShootBullet))