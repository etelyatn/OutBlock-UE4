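; FinishLevel is a trigger volume that ends the level when the player overlaps its box collision while enabled.
; It shows a FinishLevel_UI widget configured with colour, font and text.
; After a short delay it opens the named next level, or pauses the game if none is set.
; Activate, Deactivate and Switch events control whether the trigger is armed.
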(event OnComponentBeginOverlap(BoxCollision)
  (params (OverlappedComponent :type Primitive%20Component%20Object%20Reference) (OtherActor :type Actor%20Object%20Reference) (OtherComp :type Primitive%20Component%20Object%20Reference) (OtherBodyIndex :type Integer) (bFromSweep :type Boolean) (SweepResult :type Hit%20Result%20Structure%20%28by%20ref%29))
  (bind _nextlevelname (Variables|Props|GetNextLevelName))
  (Utilities|Casting|CastToPlayer OtherActor)
  (if (Variables|Props|GetEnabled)
    (CallFunction|CreateFinishLevelWidget)
    ;[0 0 0] Set Game Paused Or Load Next Level
    (if (Utilities|Name|Equal(Name) _nextlevelname "None")
      (Utilities|FlowControl|Delay 0.2)
      (Game|SetGamePaused true)
      (else
        (Utilities|FlowControl|Delay 1.0)
        (Game|OpenLevel(byName) _nextlevelname)))))

(event EventActivate
  ;[0 0 0] Activation Events
  (Variables|Props|SetEnabled true))

(event EventDeactivate
  ;[0 0 0] Activation Events
  (Variables|Props|SetEnabled false))

(event EventSwitch
  ;[0 0 0] Activation Events
  (Variables|Props|SetEnabled (not (Variables|Props|GetEnabled))))

(fn ConstructionScript)

(fn CreateFinishLevelWidget
  (bind _returnvalue (UserInterface|CreateWidget "/Game/ProjectContent/Core/Widgets/FinishLevel_UI.FinishLevel_UI_C"))
  (bind _output_get (Variables|Default|SetWidget _returnvalue))
  (UserInterface|Viewport|AddtoViewport _output_get 0)
  (Default|OnSetup _output_get (Variables|Props|UI|GetColor) (Variables|Props|UI|GetFont) (Variables|Props|UI|GetText)))