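; Hinged door actor that swings by rotating its Pivot component, with the motion supplied through UpdateDoorPosition.
; UpdateDoorPosition lerps from the Pivot's current rotation X (forward) vector to FinalPoint by Alpha, then uses the result's components as roll, pitch and yaw.
; The IsOpen input is unused, and the event graph holds only disabled stubs, so nothing here triggers the movement.
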(event EventBeginPlay
  (|CallParentFunction) ; This node is disabled and will not be called.\nDrag off pins to build functionality.
)

(event Collision|EventActorBeginOverlap
  (params (OtherActor :type Actor%20Object%20Reference))
  (|CallParentFunction OtherActor) ; This node is disabled and will not be called.\nDrag off pins to build functionality.
)

(event EventTick
  (params (DeltaSeconds :type Float%20%28single-precision%29))
  (|CallParentFunction DeltaSeconds) ; This node is disabled and will not be called.\nDrag off pins to build functionality.
)

(fn ConstructionScript
  (|CallParentFunction))

(fn UpdateDoorPosition
  (params (FinalPoint :type Vector :default "0, 0, 0") (Alpha :type Float%20%28single-precision%29) (IsOpen :type Boolean))
  (bind _pivot (Variables|Default|GetPivot))
  (bind _relativerotation (Variables|/Script/Engine.SceneComponent|GetRelativeRotation _pivot))
  (bind _returnvalue (Math|Rotator|GetRotationXVector _relativerotation))
  (bind _returnvalue_2 (Math|Vector|Lerp(Vector) _returnvalue FinalPoint Alpha))
  (Transformation|SetRelativeRotation (Variables|Default|GetPivot) (Math|Rotator|MakeRotator (.x _returnvalue_2) (.y _returnvalue_2) (.z _returnvalue_2)) false false))